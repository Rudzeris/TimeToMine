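; Ore actor that starts with durability equal to its level and is destroyed when that durability reaches zero.
; Each TakeDamage_Event calls back the sender's TakeDamageEvent, then compares the sender's level with the ore's.
; A lower-level sender needs extra hits, tracked by CountHit, per durability point, while a higher-level one removes extra points per hit.
; Remaining durability is printed as debug text after each reduction.
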(event Custom|TakeDamage_Event
  (params (sender :type BP%20Tool%20Object%20Reference))
  (bind _lvl (Variables|Default|Getlvl))
  (Default|TakeDamageEvent sender)
  (if (== (Variables|Default|GetcountHit) 0)
    (bind _lvl_2 (Default|GetLvl sender))
    (Variables|Default|SetcountHit (Math|Integer|Clamp(Integer) (- _lvl _lvl_2) 0 _lvl))
    (else
      (Math|Integer|DecrementInt (Variables|Default|GetcountHit)
        (:%20%20
          _))))
  (if (== (Variables|Default|GetcountHit) 0)
    (bind _lvl_3 (Default|GetLvl sender))
    (Variables|Default|Setdurability (Math|Integer|Clamp(Integer) (- (Variables|Default|Getdurability) (+ (Math|Integer|Clamp(Integer) (- _lvl_3 (Variables|Default|Getlvl)) 0 _lvl_3) 1)) 0 (Variables|Default|Getlvl)))
    (Development|PrintString (Utilities|String|Append "Ore durability: " (Utilities|String|ToString(Integer) (Variables|Default|Getdurability))))
    (if (== (Variables|Default|Getdurability) 0)
      (Actor|DestroyActor))))

(event EventBeginPlay
  (Variables|Default|Setdurability (Variables|Default|Getlvl)))

(event Collision|EventActorBeginOverlap
  (params (OtherActor :type Actor%20Object%20Reference)))

(event EventTick
  (params (DeltaSeconds :type Float%20%28single-precision%29)))

(fn ConstructionScript)