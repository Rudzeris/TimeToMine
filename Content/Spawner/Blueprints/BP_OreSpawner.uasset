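; BP_OreSpawner is a one-shot trigger that populates the ore spawn points inside its Box when the first-person character overlaps it.
; On BeginPlay it builds a hardcoded list of ore classes.
; On overlap it gathers BP_OreSpawnPoint actors in the Box, if none are cached, and copies its Lvl to each.
; It then shuffles them and passes the class list to a random half or more to spawn ore.
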(event EventBeginPlay
  (CallFunction|CollectionOreClasses))

(event Collision|EventActorBeginOverlap
  (params (OtherActor :type Actor%20Object%20Reference))
  (if (not (Variables|Default|GetisSpawned))
    (if (Utilities|Array|IsEmpty (Variables|Default|GetspawnPoints))
      (CallFunction|CollectionOreSpawnPoints))
    (Utilities|Casting|CastToBP_FirstPersonCharacter OtherActor)
    (Variables|Default|SetisSpawned true)
    (CallFunction|SpawnOres)))

(event EventTick
  (params (DeltaSeconds :type Float%20%28single-precision%29)))

(fn ConstructionScript)

(fn SpawnOres
  (bind _spawnpoints (Variables|Default|GetspawnPoints))
  (bind _spawnpoints_2 (Variables|Default|GetspawnPoints))
  (bind _returnvalue (Utilities|Array|Length _spawnpoints))
  (bind _output_get (LocalVariables|SetrandInt (Math|Random|RandomIntegerinRange (/ _returnvalue 2) _returnvalue)))
  (Utilities|Array|Shuffle _spawnpoints_2)
  (for _index (range 0 _output_get)
    (Utilities|IsValid (Utilities|Array|Get(acopy) _spawnpoints_2 _index)
      (:Is%20Valid
        (Default|SpawnOre (Utilities|Array|Get(acopy) _spawnpoints_2 _index) (Variables|Default|GetClasses)))))
  (Development|PrintString "Ores spawned is completed"))

(fn CollectionOreClasses
  (bind _classes (Variables|Default|GetClasses))
  (Utilities|Array|Add _classes "/Game/Ores/Blueprints/BP_Coal.BP_Coal_C")
  (Utilities|Array|Add _classes "/Game/Ores/Blueprints/BP_Copper.BP_Copper_C")
  (Utilities|Array|Add _classes "/Game/Ores/Blueprints/BP_LapisLazuri.BP_LapisLazuri_C")
  (Utilities|Array|Add _classes "/Game/Ores/Blueprints/BP_Gold.BP_Gold_C")
  (Utilities|Array|Add _classes "/Game/Ores/Blueprints/BP_RedStone.BP_RedStone_C")
  (Utilities|Array|Add _classes "/Game/Ores/Blueprints/BP_Ametist.BP_Ametist_C")
  (for _array_element _classes
    (LocalVariables|Settext (Utilities|String|Append (Utilities|String|Append (LocalVariables|Gettext) (Utilities|GetClassDisplayName _array_element)) ", ")))
  (Development|PrintString (LocalVariables|Gettext)))

(fn CollectionOreSpawnPoints
  (for _array_element (Collision|GetOverlappingActors (Variables|Default|GetBox) "/Game/Spawner/Blueprints/BP_OreSpawnPoint.BP_OreSpawnPoint_C" :!class /Script/Engine.PrimitiveComponent)
    (LocalVariables|Settext (Utilities|String|Append (Utilities|String|Append (LocalVariables|Gettext) (Utilities|GetDisplayName 0)) ", "))
    (bind _asbp_ore_spawn_point (Utilities|Casting|CastToBP_OreSpawnPoint _array_element))
    (Utilities|Array|Add (Variables|Default|GetspawnPoints) _asbp_ore_spawn_point)
    (Variables|/Game/Spawner/Blueprints/BP_OreSpawnPoint.BP_OreSpawnPoint_C|Setlvl _asbp_ore_spawn_point (Variables|Default|Getlvl)))
  (Development|PrintString (LocalVariables|Gettext)))