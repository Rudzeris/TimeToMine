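; BP_OreSpawnPoint is a spawn point that places one randomly chosen ore actor at its own location.
; SpawnOre takes an array of ore classes and spawns only when the stored Ore is invalid, then saves the new actor.
; GetRandomIndex builds thresholds scaled repeatedly by Coef and maps a random roll to an index in reverse order, weighting the pick by array position.
; Its event graph is empty, so SpawnOre relies on an external call.
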(event EventBeginPlay)

(event Collision|EventActorBeginOverlap
  (params (OtherActor :type Actor%20Object%20Reference)))

(event EventTick
  (params (DeltaSeconds :type Float%20%28single-precision%29)))

(fn ConstructionScript)

(fn SpawnOre
  (params (class%20Ore :type Array%20of%20BP%20Ore%20Class%20References))
  (if (and (not (Utilities|IsValid (Variables|Default|Getore))) (> (Utilities|Array|Length class%20Ore) 0))
    (bind _oreclass (CallFunction|GetOre class%20Ore))
    (bind _returnvalue (Game|SpawnActorfromClass _oreclass (Math|Conversions|ToTransform(Vector) (Transformation|GetActorLocation)) "Undefined" "MultiplyWithRoot" 0 0))
    (Variables|Default|Setore _returnvalue)))

(fn GetOre
  (params (oreArray :type Array%20of%20BP%20Ore%20Class%20References))
  (bind _index (CallFunction|GetRandomIndex (Utilities|Array|Length oreArray)))
  (return (Utilities|Array|Get(acopy) oreArray _index)))

(fn GetRandomIndex
  (params (maximum :type Integer))
  (bind _values (LocalVariables|Getvalues))
  (for _index (range 0 maximum)
    (Utilities|Array|Add (LocalVariables|Getvalues) (LocalVariables|Getval))
    (LocalVariables|Setval (* (LocalVariables|Getval) (LocalVariables|Getcoef))))
  (LocalVariables|Setval (Math|Random|RandomIntegerinRange 0 (Utilities|Array|Get(acopy) _values (Utilities|Array|LastIndex _values))))
  (for (_array_element _array_index) (LocalVariables|Getvalues)
    (if (> _array_element (LocalVariables|Getval))
      (return (+ (- maximum _array_index) 1))))
  (return 0))