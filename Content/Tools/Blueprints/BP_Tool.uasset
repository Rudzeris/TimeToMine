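; BP_Tool is a mining tool owned by the first-person character, with durability, repair and level upgrades.
; On BeginPlay it adds the tools input mapping and fills durability; mining line-traces from the camera and passes itself to any hit BP_Ore's damage event, gated by a speed-based cooldown.
; A separate event decrements durability.
; Repair and upgrade, available through input or events, restore durability or scale its maximum, with input presses throttled by a delay.
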(event Custom|TakeDamage_Event
  (bind _result (Math|Integer|DecrementInt (Variables|Default|Getdurability))
    (:%20%20
      (Development|PrintString (Utilities|String|Append "Tool durability: " (Utilities|String|ToString(Integer) _result))))))

(event Custom|Repar_Event
  (bind _output_get (Variables|Default|Setdurability (Variables|Default|GetmaxDurability)))
  (Development|PrintString (Utilities|String|Append "Tool repaired. Durability" (Utilities|String|ToString(Integer) _output_get)))
  (Utilities|FlowControl|Delay 1.0)
  (Variables|Default|SetisActiveInput true))

(event Custom|Upgrade_Event
  (bind _result (Math|Integer|IncrementInt (Variables|Default|Getlvl))
    (:%20%20
      (Variables|Default|SetmaxDurability (Math|Float|Truncate (* (Variables|Default|Getcoefficient) (Variables|Default|GetmaxDurability))))
      (Default|CallRepair)
      (Development|PrintString (Utilities|String|Append (Utilities|String|Append "Tool upgraded. LVL: " (Utilities|String|ToString(Integer) _result)) (Utilities|String|Append ", MaxDurability: " (Utilities|String|ToString(Integer) (Variables|Default|GetmaxDurability)))))
      (Utilities|FlowControl|Delay 1.0)
      (Variables|Default|SetisActiveInput true))))

(event Input|EnhancedActionEvents|EnhancedInputActionIA_Mine
  (params (ActionValue :type Boolean) (ElapsedSeconds :type Float%20%28double-precision%29) (TriggeredSeconds :type Float%20%28double-precision%29) (InputAction :type Input%20Action%20Object%20Reference :default "/Game/Tools/Input/IA_Mine.IA_Mine"))
  (if (and (not (Variables|Default|GetisMine)) (!= (Variables|Default|Getdurability) 0))
    (Variables|Default|SetisMine true)
    (bind _hitresult (CallFunction|LineTraceLogic))
    (bind _asbp_ore (Utilities|Casting|CastToBP_Ore (.HitActor (Collision|BreakHitResult _hitresult)))
      (:then
        (Default|TakeDamageEvent _asbp_ore self))
      (:CastFailed
        _))
    (Utilities|FlowControl|Delay (/ (Variables|Default|GetdelayMine) (Variables|Default|GetspeedMine)))
    (Variables|Default|SetisMine false)))

(event Input|EnhancedActionEvents|EnhancedInputActionIA_Repair
  (params (ActionValue :type Boolean) (ElapsedSeconds :type Float%20%28double-precision%29) (TriggeredSeconds :type Float%20%28double-precision%29) (InputAction :type Input%20Action%20Object%20Reference :default "/Game/Tools/Input/IA_Repair.IA_Repair"))
  (if (Variables|Default|GetisActiveInput)
    (Variables|Default|SetisActiveInput false)
    (bind _output_get (Variables|Default|Setdurability (Variables|Default|GetmaxDurability)))
    (Development|PrintString (Utilities|String|Append "Tool repaired. Durability" (Utilities|String|ToString(Integer) _output_get)))
    (Utilities|FlowControl|Delay 1.0)
    (Variables|Default|SetisActiveInput true)))

(event Input|EnhancedActionEvents|EnhancedInputActionIA_Upgrade
  (params (ActionValue :type Boolean) (ElapsedSeconds :type Float%20%28double-precision%29) (TriggeredSeconds :type Float%20%28double-precision%29) (InputAction :type Input%20Action%20Object%20Reference :default "/Game/Tools/Input/IA_Upgrade.IA_Upgrade"))
  (if (Variables|Default|GetisActiveInput)
    (Variables|Default|SetisActiveInput false)
    (bind _result (Math|Integer|IncrementInt (Variables|Default|Getlvl))
      (:%20%20
        (Variables|Default|SetmaxDurability (Math|Float|Truncate (* (Variables|Default|Getcoefficient) (Variables|Default|GetmaxDurability))))
        (Default|CallRepair)
        (Development|PrintString (Utilities|String|Append (Utilities|String|Append "Tool upgraded. LVL: " (Utilities|String|ToString(Integer) _result)) (Utilities|String|Append ", MaxDurability: " (Utilities|String|ToString(Integer) (Variables|Default|GetmaxDurability)))))
        (Utilities|FlowControl|Delay 1.0)
        (Variables|Default|SetisActiveInput true)))))

(event EventBeginPlay
  (bind _asbp_first_person_character (Utilities|Casting|CastToBP_FirstPersonCharacter (Components|GetOwner)))
  (bind _output_get (Variables|Default|Setcharacter _asbp_first_person_character))
  (bind _asplayer_controller (Utilities|Casting|CastToPlayerController (Pawn|GetController _output_get)))
  (Utilities|IsValid (PlayerController|LocalPlayerSubsystems|GetEnhancedInputLocalPlayerSubsystem _asplayer_controller)
    (:Is%20Valid
      (Input|AddMappingContext (PlayerController|LocalPlayerSubsystems|GetEnhancedInputLocalPlayerSubsystem _asplayer_controller) "/Game/Tools/Input/IMC_Tools.IMC_Tools" 0 "(bIgnoreAllPressedKeysUntilRelease=True,bForceImmediately=False,bNotifyUserSettings=False)")
      (Variables|Default|Setdurability (Variables|Default|GetmaxDurability)))))

(fn LineTraceLogic
  (bind _character (Variables|Default|Getcharacter))
  (bind _firstpersoncamera (Variables|/Game/FirstPerson/Blueprints/BP_FirstPersonCharacter.BP_FirstPersonCharacter_C|GetFirstPersonCamera _character))
  (bind _returnvalue (Transformation|GetWorldLocation _firstpersoncamera))
  (bind _outhit (Collision|LineTraceByChannel _returnvalue (+ _returnvalue (* (Math|Vector|GetForwardVector _firstpersoncamera) (Variables|Default|GetmineDistance))) "TraceTypeQuery2" false 0 "ForDuration"))
  (return _outhit))

(fn GetLvl
  (return (Variables|Default|Getlvl)))