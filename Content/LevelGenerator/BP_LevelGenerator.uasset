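; BP_LevelGenerator builds a linear level at BeginPlay by chaining randomly chosen module actors.
; Each module spawns at the previous one's end position, obtained through GetEndMessage, for indices zero through LevelDepth.
; BP_Wall caps the first module's start and the last module's end.
; GetRandomModule loops against LastRandomIndex but returns a fresh random roll, so repeats remain possible.
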(event EventBeginPlay
  (for _index (range 0 (Variables|Default|GetLevelDepth))
    (bind _returnvalue (Game|SpawnActorfromClass (CallFunction|GetRandomModule) (Math|Transform|MakeTransform (Variables|Default|GetEndPos) "0, 0, 0" "1.000000,1.000000,1.000000") "Undefined" "MultiplyWithRoot" 0 0))
    (bind _endpos (Class|BPIModule|GetEnd(Message) _returnvalue))
    (Variables|Default|SetEndPos _endpos)
    (Utilities|FlowControl|Sequence
      (:then_0
        (if (== _index 0)
          (bind _startpos (Class|BPIModule|GetStart(Message) _returnvalue))
          (Game|SpawnActorfromClass "/Game/LevelGenerator/BP_Wall.BP_Wall_C" (Math|Transform|MakeTransform _startpos "0, 0, 0" "1.000000,1.000000,1.000000") "Undefined" "MultiplyWithRoot" 0 0)))
      (:then_1
        (if (== _index (Variables|Default|GetLevelDepth))
          (bind _endpos_2 (Class|BPIModule|GetEnd(Message) _returnvalue))
          (Game|SpawnActorfromClass "/Game/LevelGenerator/BP_Wall.BP_Wall_C" (Math|Transform|MakeTransform _endpos_2 "0, 0, 0" "1.000000,1.000000,1.000000") "Undefined" "MultiplyWithRoot" 0 0))))))

(fn ConstructionScript)

(fn GetRandomModule
  (bind _modules (Variables|Default|GetModules))
  (bind _returnvalue (Utilities|Array|Length _modules))
  (bind _returnvalue_2 (Math|Random|RandomInteger _returnvalue))
  (while (== _returnvalue_2 (Variables|Default|GetLastRandomIndex))
    (Variables|Default|SetLastRandomIndex _returnvalue_2))
  (return (Utilities|Array|Get(acopy) _modules _returnvalue_2)))