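; BP_Rock is a level generator hazard that costs the first-person player time on contact.
; The construction script picks a random mesh from RockMeshes.
; Overlapping the player reduces the timer by Damage and plays a lava hit sound, unless the rock is flagged as IsWarning.
; A looping timer, used instead of Tick, destroys the rock once it drops below a height threshold.
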(event OnComponentBeginOverlap(RockMesh)
  (params (OverlappedComponent :type Primitive%20Component%20Object%20Reference) (OtherActor :type Actor%20Object%20Reference) (OtherComp :type Primitive%20Component%20Object%20Reference) (OtherBodyIndex :type Integer) (bFromSweep :type Boolean) (SweepResult :type Hit%20Result%20Structure%20%28by%20ref%29))
  (if (not (Variables|Default|GetIsWarning))
    (Utilities|Casting|CastToBP_FirstPersonCharacter OtherActor)
    (Default|ReduceTime (CallFunction|GetTimer) (Variables|Default|GetDamage))
    (Audio|PlaySound2D "/Game/Sound/Lava/SC_LavaHit.SC_LavaHit" 1.0 1.0 0.0 0 0)))

(event Custom|CustomTick
  (if (< (.z (Transformation|GetActorLocation)) -5e+02)
    (Actor|DestroyActor)))

(event EventBeginPlay
  (Utilities|Time|SetTimerbyEvent (delegate Custom|CustomTick) 0.1 true))

(fn ConstructionScript
  (bind _rockmeshes (Variables|Default|GetRockMeshes))
  (Components|StaticMesh|SetStaticMesh (Variables|Default|GetRockMesh) (Utilities|Array|Get(acopy) _rockmeshes (Math|Random|RandomInteger (Utilities|Array|Length _rockmeshes)))))