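; BP_Timer is a level countdown actor that counts down every second and signals when time runs out.
; A looping timer calls ReduceTime, which subtracts seconds scaled by Coef and fires the OnTimeTick or TimeIsUp dispatcher.
; The player character's OnLoadGame event sets Coef to CoefSkill when the saved Timer skill is active.
; Helpers add time and format it as minutes and zero-padded seconds.
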(event Custom|TimerHandler
  (CallFunction|ReduceTime 1)
  (Default|CallOnTimeTick))

(event Custom|OnLoadGame_Event
  (params (data :type SG%20Player%20Data%20Object%20Reference))
  (if (.timer (Variables|/Game/Save/SG_PlayerData.SG_PlayerData_C|Getskills data))
    (Variables|Default|Setcoef (Variables|Default|GetcoefSkill))))

(event EventBeginPlay
  (bind _returnvalue (Utilities|Time|SetTimerbyEvent (delegate Custom|TimerHandler) 1.0 true))
  (Variables|Default|SetTimer _returnvalue)
  (bind _returnvalue_2 (Actor|GetActorOfClass "/Game/FirstPerson/Blueprints/BP_FirstPersonCharacter.BP_FirstPersonCharacter_C"))
  (EventDispatchers|AssignOnLoadGame _returnvalue_2 (delegate Custom|OnLoadGame_Event)))

(fn ConstructionScript)

(fn GetSeconds
  (return (Math|Integer|%(Integer) (Variables|Default|GetTime) 60)))

(fn GetMinuts
  (return (/ (Variables|Default|GetTime) 60)))

(fn ReduceTime
  (params (Second :type Integer))
  (if (<= (- (Variables|Default|GetTime) (* Second (Variables|Default|Getcoef))) 0)
    (Variables|Default|SetTime (- (Variables|Default|GetTime) (* Second (Variables|Default|Getcoef))))
    (Default|CallTimeIsUp)
    (else
      (Variables|Default|SetTime (- (Variables|Default|GetTime) (* Second (Variables|Default|Getcoef))))
      (Default|CallOnTimeTick))))

(fn IncreaseTime
  (params (Second :type Integer))
  (Variables|Default|SetTime (+ (Variables|Default|GetTime) Second)))

(fn GetTimerString
  (bind _seconds (CallFunction|GetSeconds))
  (bind _minuts (CallFunction|GetMinuts))
  (bind _returnvalue (Utilities|String|ToString(Integer) _seconds))
  (bind _returnvalue_2 (Utilities|String|ToString(Integer) _seconds))
  (bind _returnvalue_3 (Utilities|String|ToString(Integer) _minuts))
  (bind _returnvalue_4 (/ _seconds 10))
  (bind _returnvalue_5 (Utilities|String|Append "0" _returnvalue_2))
  (bind _returnvalue_6 (> _returnvalue_4 0))
  (bind _returnvalue_7 (select _returnvalue_6 _returnvalue _returnvalue_5))
  (return (Utilities|String|Append _returnvalue_3 ":" _returnvalue_7) _returnvalue_3 _returnvalue_7))