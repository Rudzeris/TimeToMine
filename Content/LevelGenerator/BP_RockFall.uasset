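; BP_RockFall is a level-generator hazard that repeatedly drops rocks at random points within the inner half of its box.
; A self-restarting timer picks a randomized delay scaled by the game timer's minutes and TimeToSpawn, clamped to set bounds.
; Each cycle spawns a warning actor with sound, waits for its LifeTime, then spawns a scaled BP_Rock with sound at that spot.
; SetLvl is an empty stub.
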(event Custom|SpawnRocks
  (bind _rockscale (Variables|Default|GetRockScale))
  (bind _output_get (Variables|Default|SetRandomLoc (CallFunction|GetRandomLocationinBox)))
  (bind _returnvalue (Game|SpawnActorfromClass "/Game/LevelGenerator/BP_WarningRockFall.BP_WarningRockFall_C" (Math|Transform|MakeTransform _output_get "0, 0, 0" "1.000000,1.000000,1.000000") "Undefined" "MultiplyWithRoot" 0 0))
  (Audio|PlaySoundatLocation "/Game/Sound/RockFall/SC_WRFS.SC_WRFS" _output_get "0, 0, 0" 1.0 1.0 2.0 "/Game/Sound/RockFall/SA_Rock.SA_Rock" 0 0 0)
  (Utilities|FlowControl|Delay (Variables|/Game/LevelGenerator/BP_WarningRockFall.BP_WarningRockFall_C|GetLifeTime _returnvalue))
  (Game|SpawnActorfromClass "/Game/LevelGenerator/BP_Rock.BP_Rock_C" (Math|Transform|MakeTransform (Variables|Default|GetRandomLoc) "0, 0, 0" (Math|Vector|MakeVector _rockscale _rockscale _rockscale)) "Undefined" "MultiplyWithRoot" 0 false 50 0)
  (Audio|PlaySoundatLocation "/Game/Sound/RockFall/SC_BRS.SC_BRS" (Variables|Default|GetRandomLoc) "0, 0, 0" 1.0 1.0 0.0 "/Game/Sound/RockFall/SA_Rock.SA_Rock" 0 0 0)
  (CallFunction|RockFall))

(event Custom|RockFall
  (bind _timer (CallFunction|GetTimer))
  (bind _timetospawn (Variables|Default|GetTimeToSpawn))
  (bind _minuts (Default|GetMinuts _timer))
  (bind _returnvalue (* _minuts _timetospawn))
  (bind _returnvalue_2 (Math|Float|Clamp(Float) _returnvalue 5.0 6e+01))
  (Utilities|Time|SetTimerbyEvent (delegate Custom|SpawnRocks) (Math|Random|RandomFloatinRange (* _returnvalue_2 0.8) _returnvalue_2)))

(event EventBeginPlay
  (CallFunction|RockFall))

(fn ConstructionScript)

(fn GetRandomLocationinBox
  (bind _box (Variables|Default|GetBox))
  (bind _returnvalue (Components|Box|GetScaledBoxExtent _box))
  (return (+ (Transformation|GetActorLocation) (Math|Vector|MakeVector (Math|Random|RandomFloatinRange (/ (.x _returnvalue) -2.0) (/ (.x _returnvalue) 2.0)) (Math|Random|RandomFloatinRange (/ (.y _returnvalue) -2.0) (/ (.y _returnvalue) 2.0)) (Math|Random|RandomFloatinRange (/ (.z _returnvalue) -2.0) (/ (.z _returnvalue) 2.0))))))

(fn SetLvl
  (params (Lvl :type Float%20%28double-precision%29)))