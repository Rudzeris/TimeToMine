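; Base level-generator module that exposes Start and End connection points for placing pieces of a level.
; On BeginPlay it shifts itself in local space by the negated relative location of Start, moving its pivot-based placement toward a Start-based one.
; GetStart returns the world location of Start, while GetEnd returns the world location of End paired with its relative, not world, rotation.
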(event Custom|GetEnd_1_1)

(event EventBeginPlay
  (Transformation|AddActorLocalOffset (Math|Vector|NegateVector (Variables|/Script/Engine.SceneComponent|GetRelativeLocation (Variables|Default|GetStart))) false false))

(event Collision|EventActorBeginOverlap
  (params (OtherActor :type Actor%20Object%20Reference)))

(event EventTick
  (params (DeltaSeconds :type Float%20%28single-precision%29)))

(fn ConstructionScript)

(fn GetEnd
  (bind _end (Variables|Default|GetEnd))
  (return (Transformation|GetWorldLocation _end) (Variables|/Script/Engine.SceneComponent|GetRelativeRotation _end)))

(fn GetStart
  (return (Transformation|GetWorldLocation (Variables|Default|GetStart))))