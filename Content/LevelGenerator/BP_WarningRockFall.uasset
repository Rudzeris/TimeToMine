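; BP_WarningRockFall is a temporary level actor that drops small warning rocks, apparently to signal a rockfall.
; On BeginPlay it sets its lifespan and starts a looping half-second timer that spawns a random handful of tiny BP_Rock actors flagged IsWarning.
; GetRandomLocationInBox picks points around the actor within half the Box extent on each axis.
; A second random point, converted through RotationFromXVector, supplies each rock's rotation.
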(event Custom|SpawnRocks
  (bind _returnvalue (CallFunction|GetRandomLocationinBox))
  (for _index (range 0 (Math|Random|RandomIntegerinRange 2 5))
    (Game|SpawnActorfromClass "/Game/LevelGenerator/BP_Rock.BP_Rock_C" (Math|Transform|MakeTransform _returnvalue (Math|Conversions|RotationFromXVector _returnvalue) "0.030000,0.030000,0.030000") "Undefined" "MultiplyWithRoot" 0 true 0)))

(event EventBeginPlay
  (Actor|SetLifeSpan (Variables|Default|GetLifeTime))
  (Utilities|Time|SetTimerbyEvent (delegate Custom|SpawnRocks) 0.5 true))

(fn ConstructionScript)

(fn GetRandomLocationinBox
  (bind _box (Variables|Default|GetBox))
  (bind _returnvalue (Components|Box|GetScaledBoxExtent _box))
  (return (+ (Transformation|GetActorLocation) (Math|Vector|MakeVector (Math|Random|RandomFloatinRange (/ (.x _returnvalue) -2.0) (/ (.x _returnvalue) 2.0)) (Math|Random|RandomFloatinRange (/ (.y _returnvalue) -2.0) (/ (.y _returnvalue) 2.0)) (Math|Random|RandomFloatinRange (/ (.z _returnvalue) -2.0) (/ (.z _returnvalue) 2.0))))))